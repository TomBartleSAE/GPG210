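; ScoreManager is an actor Blueprint that displays the first-person player's score as debug text.
; On BeginPlay it finds the FirstPersonCharacter, stores it as Player and binds ShowScore to that character's AddScoreEvent dispatcher.
; Each broadcast prints the Player's current Score with PrintString, and the binding is removed when the manager is destroyed.
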(event Custom|ShowScore
  ;[1 1 1] Show score
  (Development|PrintString (Utilities|String|ToString(Integer) (Variables|/Game/FirstPersonBP/Blueprints/FirstPersonCharacter.FirstPersonCharacter_C|GetScore (Variables|Default|GetPlayer)))))

(event EventBeginPlay
  ;[1 1 1] Subscribe to event
  (bind _returnvalue (Actor|GetActorOfClass "/Game/FirstPersonBP/Blueprints/FirstPersonCharacter.FirstPersonCharacter_C"))
  (bind _output_get (Variables|Default|SetPlayer _returnvalue))
  (EventDispatchers|BindEventtoAddScoreEvent _output_get (delegate Custom|ShowScore)))

(event EventDestroyed
  ;[1 1 1] Unsubscribe from event
  (EventDispatchers|UnbindEventfromAddScoreEvent (Variables|Default|GetPlayer) (delegate Custom|ShowScore)))

(fn ConstructionScript)