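; Meteor spawner actor that periodically spawns Meteor actors until a 60-second timer from BeginPlay sets StopSpawning.
; Tick paces spawning through a Delay of SpawnDelay (noted as two seconds) instead of a looping timer.
; Each meteor takes the spawner's X and Z, a random absolute world Y, and a randomized pitch.
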(event EventBeginPlay
  ;[1 1 1] Stop spawning meteors after 60 seconds
  (Utilities|FlowControl|Delay 6e+01)
  (Variables|Default|SetStopSpawning true))

(event EventTick
  (params (DeltaSeconds :type Float%20%28single-precision%29))
  (bind _returnvalue (Transformation|GetActorLocation))
  ;[1 1 1] Spawn meteor every 2 seconds, give it random position
  (if (not (Variables|Default|GetStopSpawning))
    (Utilities|FlowControl|Delay (Variables|Default|GetSpawnDelay))
    (Game|SpawnActorfromClass "/Game/Blueprints/Meteor.Meteor_C" (Math|Transform|MakeTransform (Math|Vector|MakeVector (.x _returnvalue) (Math|Random|RandomFloatinRange -2e+03 2e+03) (.z _returnvalue)) (Math|Rotator|MakeRotator 9e+01 (Math|Random|RandomFloatinRange -45.0 -135.0) 9e+01)) "Undefined" 0 0)))

(fn ConstructionScript)